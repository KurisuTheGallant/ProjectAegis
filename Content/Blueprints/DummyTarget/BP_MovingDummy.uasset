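; BP_MovingDummy is a target dummy that moves toward a start or end location while it is alive.
; Each Tick it checks IsDead, then uses the MovingToEnd flag to pick StartLocation or EndLocation as the destination.
; VInterpTo eases the actor there at MovementSpeed without sweeping, and this file never toggles the direction flag.
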(event `self.ReceiveTick`
  (params (DeltaSeconds :type "Float (single-precision)"))
  (if (`self.IsDead`)
    _
    (elif (`self.bMovingToEnd`)
      (`self.K2_SetActorLocation` (`KismetMathLibrary.VInterpTo` (`self.K2_GetActorLocation`) (`self.EndLocation`) DeltaSeconds (`self.MovementSpeed`)))
      (else
        (`self.K2_SetActorLocation` (`KismetMathLibrary.VInterpTo` (`self.K2_GetActorLocation`) (`self.StartLocation`) DeltaSeconds (`self.MovementSpeed`)))))))

(fn `UserConstructionScript`)